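; LibraryCardBP is a card actor for the library that shows its artwork and opens a preview when clicked.
; The construction script looks up a texture by Path through the Asset Registry and applies it to Art via a dynamic material instance.
; Hovering the Box shows a glow and enables input.
; A click, or right-click while hovered, adds a CardPreviewBP widget with that texture, flagged as in-library.
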(event OnBeginCursorOver(Box)
  (params (TouchedComponent :type Primitive%20Component%20Object%20Reference))
  (Variables|Default|SetHovered true)
  (Rendering|SetVisibility (Variables|Components|GetGlow) true false)
  (Input|EnableInput (Game|GetPlayerController 0)))

(event OnEndCursorOver(Box)
  (params (TouchedComponent :type Primitive%20Component%20Object%20Reference))
  (Variables|Default|SetHovered false)
  (Rendering|SetVisibility (Variables|Components|GetGlow) false false)
  (Input|DisableInput 0))

(event OnClicked(Box)
  (params (TouchedComponent :type Primitive%20Component%20Object%20Reference) (ButtonPressed :type Key%20Structure :default "None"))
  (CallFunction|PreviewCard)
  (Variables|Default|SetHovered false))

(event EventBeginPlay)

(event Collision|EventActorBeginOverlap
  (params (OtherActor :type Actor%20Object%20Reference)))

(event EventTick
  (params (DeltaSeconds :type Float%20%28single-precision%29)))

(event Input|MouseEvents|RightMouseButton
  (params (Key :type Key%20Structure :default "None"))
  (:Pressed
    (if (Variables|Default|GetHovered)
      (CallFunction|PreviewCard)
      (Variables|Default|SetHovered false))))

(fn ConstructionScript
  (bind _returnvalue (Rendering|Material|CreateDynamicMaterialInstance (Variables|Components|GetArt) 0 "/Game/Materials/CardMat.CardMat" "None" :!class /Script/Engine.PrimitiveComponent))
  (bind _returnvalue_2 (Class|AssetRegistry|GetAssetbyObjectPath (Class|AssetRegistryHelpers|GetAssetRegistry) (Utilities|MakeSoftObjectPath (Variables|Default|GetPath)) false true))
  (bind _astexture_2d (Utilities|Casting|CastToTexture2D (Class|AssetRegistryHelpers|GetAsset _returnvalue_2)))
  (bind _output_get (Variables|Default|SetTexture _astexture_2d))
  (Rendering|Material|SetTextureParameterValue _returnvalue "Texture" _output_get)
  (Rendering|Material|SetMaterial (Variables|Components|GetArt) 0 _returnvalue)
  (Input|DisableInput 0))

(fn PreviewCard
  (bind _returnvalue (UserInterface|CreateWidget "/Game/Blueprints/CardPreviewBP.CardPreviewBP_C"))
  (Appearance|SetBrushfromTexture (Variables|/Game/Blueprints/CardPreviewBP.CardPreviewBP_C|GetCard _returnvalue) (Variables|Default|GetTexture) false)
  (Variables|/Game/Blueprints/CardPreviewBP.CardPreviewBP_C|SetInLibrary _returnvalue true)
  (UserInterface|Viewport|AddtoViewport _returnvalue 0))