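; DeckBP is a clickable card deck that deals cards into the player's hand.
; Shortly after BeginPlay it fills DeckCards from the actors overlapping it, so its contents come from placement in the level.
; Clicking its Collision takes the last card, snaps it to the player's HandPivot and passes it to the player's AddCard.
; Hover events only print debug text, and an older attached-actor draw approach remains unwired.
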(event OnClicked(Collision)
  (params (TouchedComponent :type Primitive%20Component%20Object%20Reference) (ButtonPressed :type Key%20Structure :default "None"))
  (bind _deckcards (Variables|Default|GetDeckCards))
  (if (not (Utilities|Array|IsEmpty _deckcards))
    (bind _ascard_bp (Utilities|Casting|CastToCardBP (Utilities|Array|Get(acopy) _deckcards (Utilities|Array|LastIndex _deckcards))))
    (bind _output_get (Variables|Default|SetClickedCard _ascard_bp))
    (Transformation|AttachComponentToComponent _output_get (Variables|/Game/Blueprints/PlayerBP.PlayerBP_C|GetHandPivot (Variables|Default|GetPlayer)) "None" "SnapToTarget" "SnapToTarget" "KeepRelative" true)
    (Utilities|Array|RemoveItem (Variables|Default|GetDeckCards) (Variables|Default|GetClickedCard))
    (Default|AddCard (Variables|Default|GetPlayer) (Variables|Default|GetClickedCard))))

(event OnBeginCursorOver(Collision)
  (params (TouchedComponent :type Primitive%20Component%20Object%20Reference))
  (Development|PrintString "Enter Deck"))

(event OnEndCursorOver(Collision)
  (params (TouchedComponent :type Primitive%20Component%20Object%20Reference))
  (Development|PrintString "Exit Deck"))

(event EventBeginPlay
  (bind _deckcards (Variables|Default|GetDeckCards))
  (Utilities|FlowControl|Delay 0.1)
  (for _array_element (Collision|GetOverlappingActors 0 :!class /Script/Engine.Actor)
    (Utilities|Array|Add (Variables|Default|GetDeckCards) _array_element))
  (for _array_element_2 _deckcards
    (Development|PrintString (Utilities|GetDisplayName _array_element_2)))
  (Development|PrintString (Utilities|String|ToString(Integer) (Utilities|Array|Length _deckcards))))

(event Collision|EventActorBeginOverlap
  (params (OtherActor :type Actor%20Object%20Reference)))

(event EventTick
  (params (DeltaSeconds :type Float%20%28single-precision%29)))

(fn ConstructionScript)