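; CardBP1 is a card actor that takes a random texture from CardArtPath as its art and responds to the mouse.
; BeginPlay applies the texture to Art through a dynamic material instance.
; Hovering an unplaced, unselected card offsets its Base and enables input, while clicking passes the card to Player.SelectCard.
; Right-clicking a hovered card opens a CardPreviewBP widget with the same art, with a Player flag blocking simultaneous previews.
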(event OnBeginCursorOver(Box)
  (params (TouchedComponent :type Primitive%20Component%20Object%20Reference))
  (if (Math|Boolean|ANDBoolean (not (Variables|Default|GetSelected)) (not (Variables|Default|GetPlaced)) (not (== (Variables|Default|GetPlayer) 0)))
    (Transformation|AddLocalOffset (Variables|Default|GetBase) "20.000000,0.000000,0.000000" false false)
    (Variables|Default|SetHovered true)
    (Input|EnableInput (Game|GetPlayerController 0))))

(event OnClicked(Box)
  (params (TouchedComponent :type Primitive%20Component%20Object%20Reference) (ButtonPressed :type Key%20Structure))
  (if (and (not (Variables|Default|GetPlaced)) (not (== (Variables|Default|GetPlayer) 0)))
    (Default|SelectCard (Variables|Default|GetPlayer) self)))

(event OnEndCursorOver(Box)
  (params (TouchedComponent :type Primitive%20Component%20Object%20Reference))
  (if (Math|Boolean|ANDBoolean (not (Variables|Default|GetSelected)) (not (Variables|Default|GetPlaced)) (not (== (Variables|Default|GetPlayer) 0)))
    (Transformation|AddLocalOffset (Variables|Default|GetBase) "-20.000000,0.000000,0.000000" false false)
    (Variables|Default|SetHovered false)
    (Input|DisableInput 0)))

(event EventBeginPlay
  (bind _returnvalue (Rendering|Material|CreateDynamicMaterialInstance (Variables|Default|GetArt) 0 "/Game/Materials/CardMat.CardMat" "None" :!class /Script/Engine.PrimitiveComponent))
  (bind _outassetdata (Class|AssetRegistry|GetAssetsbyPath (Class|AssetRegistryHelpers|GetAssetRegistry) (Utilities|String|StringToName (Variables|Default|GetCardArtPath)) false false))
  (bind _astexture_2d (Utilities|Casting|CastToTexture2D (Class|AssetRegistryHelpers|GetAsset (.OutItem (Utilities|Array|Random _outassetdata)))))
  (Rendering|Material|SetTextureParameterValue _returnvalue "Texture" _astexture_2d)
  (Rendering|Material|SetMaterial (Variables|Default|GetArt) 0 _returnvalue)
  (Variables|Default|SetTexture _astexture_2d)
  (Input|DisableInput 0))

(event Collision|EventActorBeginOverlap
  (params (OtherActor :type Actor%20Object%20Reference)))

(event EventTick
  (params (DeltaSeconds :type Float%20%28single-precision%29)))

(event Input|MouseEvents|RightMouseButton
  (params (Key :type Key%20Structure))
  (:Pressed
    (if (Math|Boolean|ANDBoolean (Variables|Default|GetHovered) (not (Variables|Default|GetPreviewing)) (not (Variables|/Game/Blueprints/PlayerBP.PlayerBP_C|GetPreviewing (Variables|Default|GetPlayer))))
      (CallFunction|PreviewCard)
      (Variables|Default|SetPreviewing true)
      (Variables|/Game/Blueprints/PlayerBP.PlayerBP_C|SetPreviewing (Variables|Default|GetPlayer) true)
      (Variables|Default|SetHovered false))))

(fn ConstructionScript)

(fn PreviewCard
  (bind _returnvalue (UserInterface|CreateWidget "/Game/Blueprints/CardPreviewBP.CardPreviewBP_C"))
  (Variables|/Game/Blueprints/CardPreviewBP.CardPreviewBP_C|SetCardActor _returnvalue self)
  (Appearance|SetBrushfromTexture (Variables|/Game/Blueprints/CardPreviewBP.CardPreviewBP_C|GetCard _returnvalue) (Variables|Default|GetTexture) false)
  (UserInterface|Viewport|AddtoViewport _returnvalue 0))