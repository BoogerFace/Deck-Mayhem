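; Battle manager for a lane-based card game, resolving the battle phase one player-versus-enemy lane at a time, then ending the phase.
; Each occupied lane plays a mirrored timeline lunge, then chains trigger checks, card damage and Blood damage from attack exceeding opposing defense.
; The chain self-advances only past missing cards, so valid cards must resume it externally.
; Depleted Blood loads the win or lose level, while a draw only prints.
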(event Custom|Lane%20Battle
  (bind _playerslots (Variables|Default|GetPlayerSlots))
  (bind _enemyslots (Variables|Default|GetEnemySlots))
  (bind _currentlane (Variables|Default|GetCurrentLane))
  (bind _currentlane_2 (Variables|Default|GetCurrentLane))
  (bind _output (Utilities|Array|Get(acopy) _enemyslots _currentlane_2))
  (bind _output_2 (Utilities|Array|Get(acopy) _playerslots _currentlane))
  (bind _placedcard (Variables|/Game/Blueprints/SlotBP.SlotBP_C|GetPlacedCard _output_2))
  (bind _placedcard_2 (Variables|/Game/Blueprints/SlotBP.SlotBP_C|GetPlacedCard _output))
  (Variables|/Game/Blueprints/PlayerBP.PlayerBP_C|SetIsBattling (Variables|Default|GetPlayer) true)
  (Development|PrintString (Utilities|String|Append "Lane " (Utilities|String|ToString(Integer) (Variables|Default|GetCurrentLane)) " battling..."))
  (Utilities|IsValid _placedcard
    (:Is%20Valid
      (bind _output_get (Variables|Default|SetPlayerCard _placedcard))
      (Variables|Default|SetPCardStats (Variables|/Game/Blueprints/CardBP.CardBP_C|GetStats _output_get)))
    (:Is%20Not%20Valid
      _))
  (Utilities|IsValid _placedcard_2
    (:Is%20Valid
      (bind _output_get_2 (Variables|Default|SetEnemyCard _placedcard_2))
      (Variables|Default|SetECardStats (Variables|/Game/Blueprints/CardBP.CardBP_C|GetStats _output_get_2)))
    (:Is%20Not%20Valid
      _))
  (if (or (Utilities|IsValid (Variables|Default|GetPlayerCard)) (Utilities|IsValid (Variables|Default|GetEnemyCard)))
    (CallFunction|PlayAnimation)
    (else
      (CallFunction|NextLane))))

(event Custom|StartBattle
  (bind _player (Variables|Default|GetPlayer))
  (if (Math|Boolean|ANDBoolean (not (Variables|/Game/Blueprints/PlayerBP.PlayerBP_C|GetIsBattling _player)) (not (Variables|/Game/Blueprints/PlayerBP.PlayerBP_C|GetIsPlacingCard _player)) (not (Variables|/Game/Blueprints/DeckBP.DeckBP_C|GetIsDrawing (Variables|/Game/Blueprints/PlayerBP.PlayerBP_C|GetDeck _player))))
    (CallFunction|LaneBattle)))

(event Custom|CheckEnemyCardDamage
  (Utilities|IsValid (Variables|Default|GetEnemyCard)
    (:Is%20Valid
      (Default|TakeDamage (Variables|Default|GetEnemyCard) (.attack (Variables|Default|GetPCardStats))))
    (:Is%20Not%20Valid
      (CallFunction|CheckHealthDamage))))

(event Custom|CheckHealthDamage
  (if (> (- (.attack (Variables|Default|GetECardStats)) (.defense (Variables|Default|GetPCardStats))) 0)
    (Variables|/Game/Blueprints/PlayerBP.PlayerBP_C|SetBlood (Variables|Default|GetPlayer) (- (Variables|/Game/Blueprints/PlayerBP.PlayerBP_C|GetBlood (Variables|Default|GetPlayer)) (- (.attack (Variables|Default|GetECardStats)) (.defense (Variables|Default|GetPCardStats))))))
  (if (> (- (.attack (Variables|Default|GetPCardStats)) (.defense (Variables|Default|GetECardStats))) 0)
    (Variables|/Game/Blueprints/PlayerBP.PlayerBP_C|SetEnemyBlood (Variables|Default|GetPlayer) (- (Variables|/Game/Blueprints/PlayerBP.PlayerBP_C|GetEnemyBlood (Variables|Default|GetPlayer)) (- (.attack (Variables|Default|GetPCardStats)) (.defense (Variables|Default|GetECardStats))))))
  (Rendering|Components|TextRender|SetText (Variables|/Game/Blueprints/PlayerBP.PlayerBP_C|GetBloodUI (Variables|Default|GetPlayer)) (Utilities|Text|ToText(String) (Utilities|String|Append "Blood: " (Utilities|String|ToString(Integer) (Variables|/Game/Blueprints/PlayerBP.PlayerBP_C|GetBlood (Variables|Default|GetPlayer))))))
  (Rendering|Components|TextRender|SetText (Variables|/Game/Blueprints/PlayerBP.PlayerBP_C|GetEnemyBloodUI (Variables|Default|GetPlayer)) (Utilities|Text|ToText(String) (Utilities|String|Append "Enemy: " (Utilities|String|ToString(Integer) (Variables|/Game/Blueprints/PlayerBP.PlayerBP_C|GetEnemyBlood (Variables|Default|GetPlayer))))))
  (Variables|Default|SetPlayerCard 0)
  (Variables|Default|SetEnemyCard 0)
  (Variables|Default|SetPCardStats "")
  (Variables|Default|SetECardStats "")
  (if (and (<= (Variables|/Game/Blueprints/PlayerBP.PlayerBP_C|GetEnemyBlood (Variables|Default|GetPlayer)) 0) (<= (Variables|/Game/Blueprints/PlayerBP.PlayerBP_C|GetBlood (Variables|Default|GetPlayer)) 0))
    (Development|PrintString "Draw")
    (elif (<= (Variables|/Game/Blueprints/PlayerBP.PlayerBP_C|GetEnemyBlood (Variables|Default|GetPlayer)) 0)
      (Development|PrintString "Win")
      (Game|OpenLevel(byObjectReference) "/Game/Maps/WinScreen.WinScreen")
      (elif (<= (Variables|/Game/Blueprints/PlayerBP.PlayerBP_C|GetBlood (Variables|Default|GetPlayer)) 0)
        (Development|PrintString "Lose")
        (Game|OpenLevel(byObjectReference) "/Game/Maps/LoseScreen.LoseScreen")
        (else
          (CallFunction|NextLane))))))

(event Custom|CheckPlayerCardDamage
  (Utilities|IsValid (Variables|Default|GetPlayerCard)
    (:Is%20Valid
      (Default|TakeDamage (Variables|Default|GetPlayerCard) (.attack (Variables|Default|GetECardStats))))
    (:Is%20Not%20Valid
      (CallFunction|CheckEnemyCardDamage))))

(event Custom|PlayAnimation
  (Variables|Default|SetBattlePosMin "-40.000000,0.000000,0.000000")
  (Variables|Default|SetBattlePosMax "40.000000,0.000000,20.000000")
  (bind (_direction _xpos _zpos) (Timeline|BattleAnim PlayFromStart)
    (:Update
      (Utilities|FlowControl|Sequence
        (:then_0
          (Utilities|IsValid (Variables|Default|GetPlayerCard)
            (:Is%20Valid
              (Transformation|SetActorRelativeLocation (Variables|Default|GetPlayerCard) (Math|Vector|MakeVector (Math|Float|Lerp (.x (Variables|Default|GetBattlePosMin)) (.x (Variables|Default|GetBattlePosMax)) _xpos) 0.0 (Math|Float|Lerp (.z (Variables|Default|GetBattlePosMin)) (.z (Variables|Default|GetBattlePosMax)) _zpos))) ; Player Card Animation
            )))
        (:then_1
          (Utilities|IsValid (Variables|Default|GetEnemyCard)
            (:Is%20Valid
              (Transformation|SetActorRelativeLocation (Variables|Default|GetEnemyCard) (Math|Vector|MakeVector (* (Math|Float|Lerp (.x (Variables|Default|GetBattlePosMin)) (.x (Variables|Default|GetBattlePosMax)) _xpos) -1.0) 0.0 (Math|Float|Lerp (.z (Variables|Default|GetBattlePosMin)) (.z (Variables|Default|GetBattlePosMax)) _zpos))) ; Enemy Card Animation
            )))))
    (:Finished
      (CallFunction|PlayerCardCheckEffect))))

(event Custom|NextLane
  (bind _phasemanager (Variables|Default|GetPhaseManager))
  (Math|Integer|IncrementInt (Variables|Default|GetCurrentLane) ; Loop
    (:%20%20
      (if (< (Variables|Default|GetCurrentLane) (Utilities|Array|Length (Variables|Default|GetPlayerSlots)))
        (CallFunction|LaneBattle)
        (else
          (Variables|Default|SetCurrentLane 0)
          (Variables|/Game/Blueprints/PlayerBP.PlayerBP_C|SetIsBattling (Variables|Default|GetPlayer) false)
          (Variables|/Game/Blueprints/PhaseManagerBP.PhaseManagerBP_C|SetCurrentPhase _phasemanager "NewEnumerator3")
          (Default|EndPhase _phasemanager))))))

(event Custom|PlayerCardCheckEffect
  (bind _playercard (Variables|Default|GetPlayerCard))
  (Utilities|IsValid _playercard
    (:Is%20Valid
      (Default|CheckTriggers _playercard "NewEnumerator2"))
    (:Is%20Not%20Valid
      (CallFunction|EnemyCardCheckEffect))))

(event Custom|EnemyCardCheckEffect
  (bind _enemycard (Variables|Default|GetEnemyCard))
  (Utilities|IsValid _enemycard
    (:Is%20Valid
      (Default|CheckTriggers _enemycard "NewEnumerator2"))
    (:Is%20Not%20Valid
      (CallFunction|CheckPlayerCardDamage))))

(event EventBeginPlay)

(event Collision|EventActorBeginOverlap
  (params (OtherActor :type Actor%20Object%20Reference)))

(event EventTick
  (params (DeltaSeconds :type Float%20%28single-precision%29)))

(fn ConstructionScript)