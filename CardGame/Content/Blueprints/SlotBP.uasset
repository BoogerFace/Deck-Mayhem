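; SlotBP is a card slot in a turn-based card game that receives cards from the player's hand and previews placed ones.
; Hovering its Box toggles a glow and enables input on the slot only while the cursor is over it.
; Clicking an empty player-side slot calls Player.PlaceCard with the selected card, gated by turn, phase and battle state.
; Right-clicking a hovered, occupied slot previews its card.
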(event OnBeginCursorOver(Box)
  (params (TouchedComponent :type Primitive%20Component%20Object%20Reference))
  (Rendering|SetVisibility (Variables|Default|GetGlow) true false)
  (Variables|Default|SetHovered true)
  (Input|EnableInput (Game|GetPlayerController 0)))

(event OnEndCursorOver(Box)
  (params (TouchedComponent :type Primitive%20Component%20Object%20Reference))
  (Rendering|SetVisibility (Variables|Default|GetGlow) false false)
  (Variables|Default|SetHovered false)
  (Input|DisableInput 0))

(event OnClicked(Box)
  (params (TouchedComponent :type Primitive%20Component%20Object%20Reference) (ButtonPressed :type Key%20Structure :default "None"))
  (bind _player (Variables|Default|GetPlayer))
  (bind _currentcard (Variables|/Game/Blueprints/PlayerBP.PlayerBP_C|GetCurrentCard _player))
  (if (Math|Boolean|ANDBoolean (Variables|Default|GetPlayerSide) (not (Variables|/Game/Blueprints/PlayerBP.PlayerBP_C|GetIsBattling (Variables|Default|GetPlayer))) (Variables|/Game/Blueprints/PhaseManagerBP.PhaseManagerBP_C|GetIsPlayerTurn (Variables|Default|GetPhaseManager)) (Utilities|Enum|Equal(Enum) (Variables|/Game/Blueprints/PhaseManagerBP.PhaseManagerBP_C|GetCurrentPhase (Variables|Default|GetPhaseManager)) "NewEnumerator1"))
    (if (and (== (Variables|Default|GetPlacedCard) 0) (Utilities|IsValid _currentcard)) ; Check if there is not already\na card in slot, AND if a card\nis selected in hand
      (Development|PrintString (Utilities|GetDisplayName _currentcard))
      (Default|PlaceCard _player self))))

(event EventBeginPlay)

(event Collision|EventActorBeginOverlap
  (params (OtherActor :type Actor%20Object%20Reference)))

(event EventTick
  (params (DeltaSeconds :type Float%20%28single-precision%29)))

(event Input|MouseEvents|RightMouseButton
  (params (Key :type Key%20Structure :default "None"))
  (bind _placedcard (Variables|Default|GetPlacedCard))
  (:Pressed
    (if (and (Variables|Default|GetHovered) (not (== (Variables|Default|GetPlacedCard) 0)))
      (Default|PreviewCard _placedcard)
      (Variables|/Game/Blueprints/CardBP.CardBP_C|SetPreviewing _placedcard true)
      (Variables|/Game/Blueprints/PlayerBP.PlayerBP_C|SetPreviewing (Variables|Default|GetPlayer) true))))

(fn ConstructionScript)