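; Turn and phase manager for a card battle game, alternating player and enemy through draw, main, battle and end phases.
; Timed delays pace the flow, announced by a colored banner sliding across the UI, while decks and BattleManager handle draws and combat.
; On enemy turns it places a random hand card in a random free slot.
; Turn switches check board cards' triggers one index at a time, pausing at each occupied slot.
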(event Custom|DrawPhase
  (if (Variables|Default|GetIsPlayerTurn)
    (CallFunction|PhaseTransition "(R=0.000000,G=0.500000,B=1.000000,A=1.000000)" "Draw Phase")
    (Utilities|FlowControl|Delay 1.2)
    (Development|PrintString "Draw Phase")
    (Variables|Default|SetCurrentPhase "NewEnumerator0")
    (Default|DrawCard (Variables|Default|GetPlayerDeck))
    (else
      (CallFunction|PhaseTransition "(R=1.000000,G=0.000000,B=0.000000,A=1.000000)" "Draw Phase")
      (Utilities|FlowControl|Delay 1.2)
      (Development|PrintString "Draw Phase")
      (Variables|Default|SetCurrentPhase "NewEnumerator0")
      (Default|DrawCard (Variables|Default|GetEnemyDeck)))))

(event Custom|MainPhase
  (if (Variables|Default|GetIsPlayerTurn)
    (CallFunction|PhaseTransition "(R=0.000000,G=0.500000,B=1.000000,A=1.000000)" "Main Phase")
    (Utilities|FlowControl|Delay 1.2)
    (Development|PrintString "Main Phase")
    (Variables|Default|SetCurrentPhase "NewEnumerator1")
    (else
      (CallFunction|PhaseTransition "(R=1.000000,G=0.000000,B=0.000000,A=1.000000)" "Main Phase")
      (Utilities|FlowControl|Delay 1.2)
      (Development|PrintString "Main Phase")
      (Variables|Default|SetCurrentPhase "NewEnumerator1")
      (Utilities|FlowControl|Delay 1.2)
      (CallFunction|AIPlayCard)
      (Utilities|FlowControl|Delay 2.4)
      (CallFunction|BattlePhase))))

(event Custom|BattlePhase
  (if (Utilities|Enum|Equal(Enum) (Variables|Default|GetCurrentPhase) "NewEnumerator1")
    (if (Variables|Default|GetIsPlayerTurn)
      (CallFunction|PhaseTransition "(R=0.000000,G=0.500000,B=1.000000,A=1.000000)" "Battle Phase")
      (else
        (CallFunction|PhaseTransition "(R=1.000000,G=0.000000,B=0.000000,A=1.000000)" "Battle Phase")))
    (Development|PrintString "Batttle Phase")
    (Variables|Default|SetCurrentPhase "NewEnumerator2")
    (Utilities|FlowControl|Delay 1.2)
    (Default|StartBattle (Variables|Default|GetBattleManager))))

(event Custom|EndPhase
  (if (Variables|Default|GetIsPlayerTurn)
    (CallFunction|PhaseTransition "(R=0.000000,G=0.500000,B=1.000000,A=1.000000)" "End Phase")
    (else
      (CallFunction|PhaseTransition "(R=1.000000,G=0.000000,B=0.000000,A=1.000000)" "End Phase")))
  (Development|PrintString "End Phase")
  (Variables|Default|SetCurrentPhase "NewEnumerator3")
  (Utilities|FlowControl|Delay 1.2)
  (CallFunction|SwitchTurn))

(event Custom|SwitchTurn
  (Variables|Default|SetIsPlayerTurn (not (Variables|Default|GetIsPlayerTurn)))
  (if (Variables|Default|GetIsPlayerTurn)
    (CallFunction|PhaseTransition "(R=0.000000,G=0.500000,B=1.000000,A=1.000000)" "Player Turn")
    (else
      (CallFunction|PhaseTransition "(R=1.000000,G=0.000000,B=0.000000,A=1.000000)" "Enemy Turn")))
  (Development|PrintString "Switch Turn")
  (Utilities|FlowControl|Delay 1.2)
  (CallFunction|CheckonStartEffects))

(event Custom|PhaseTransition
  (params (Color :type Linear%20Color%20Structure :default "(R=1.000000,G=1.000000,B=1.000000,A=1.000000)") (Text :type Text))
  (bind _phase_border (Variables|Default|GetPhase%20Border))
  (bind _phase_text (Variables|Default|GetPhase%20Text))
  (Appearance|SetColorandOpacity _phase_text (Utilities|Struct|MakeSlateColor Color "UseColor_Specified") :!class /Script/UMG.TextBlock)
  (Rendering|Components|TextRender|SetText _phase_text Text)
  (Widget|SetVisibility (Variables|Default|GetPhase%20Border) "Visible")
  (bind _float (Timeline|Timeline PlayFromStart)
    (:Update
      (Class|Widget|SetRenderTranslation _phase_border (Math|Vector2D|MakeVector2D (Math|Float|Lerp -1.92e+03 1.92e+03 _float) 0.0)))
    (:Finished
      (Widget|SetVisibility _phase_border "Hidden"))))

(event Custom|FinishSwitchTurn
  (CallFunction|DrawPhase)
  (Variables|Default|SetCurrentCardIndex 0))

(event Custom|CheckOnStartEffects
  (bind _playerslots (Variables|Default|GetPlayerSlots))
  (bind _currentcardindex (Variables|Default|GetCurrentCardIndex))
  (bind _output (Utilities|Array|Get(acopy) _playerslots _currentcardindex))
  (bind _placedcard (Variables|/Game/Blueprints/SlotBP.SlotBP_C|GetPlacedCard _output))
  (if (< (Variables|Default|GetCurrentCardIndex) 10)
    (if (< (Variables|Default|GetCurrentCardIndex) 5)
      (Utilities|IsValid _placedcard
        (:Is%20Valid
          (Default|CheckTriggers _placedcard "NewEnumerator1")
          (Math|Integer|IncrementInt (Variables|Default|GetCurrentCardIndex)))
        (:Is%20Not%20Valid
          (Math|Integer|IncrementInt (Variables|Default|GetCurrentCardIndex)
            (:%20%20
              (CallFunction|CheckonStartEffects)))))
      (else
        (Utilities|IsValid 0
          (:Is%20Valid
            (Default|CheckTriggers (Variables|/Game/Blueprints/SlotBP.SlotBP_C|GetPlacedCard (Utilities|Array|Get(acopy) (Variables|Default|GetEnemySlots) (- (Variables|Default|GetCurrentCardIndex) 5))) "NewEnumerator1")
            (Math|Integer|IncrementInt (Variables|Default|GetCurrentCardIndex)))
          (:Is%20Not%20Valid
            (Math|Integer|IncrementInt (Variables|Default|GetCurrentCardIndex)
              (:%20%20
                (CallFunction|CheckonStartEffects)))))))
    (else
      (CallFunction|FinishSwitchTurn))))

(event Custom|StartPhase
  (bind _player (Variables|Default|GetPlayer))
  (bind _ui (Variables|/Game/Blueprints/PlayerBP.PlayerBP_C|GetUI _player))
  (Variables|Default|SetCurrentPhase "NewEnumerator5")
  (Development|PrintString "Start Phase")
  (Variables|Default|SetPhase%20Text (Variables|/Game/Blueprints/UI/GameUIBP.GameUIBP_C|GetPhaseText _ui))
  (Variables|Default|SetPhase%20Border (Variables|/Game/Blueprints/UI/GameUIBP.GameUIBP_C|GetPhaseBorder _ui))
  (CallFunction|PhaseTransition "(R=1.000000,G=1.000000,B=1.000000,A=1.000000)" "Battle Start")
  (Utilities|FlowControl|Delay 0.2)
  (Default|StartDraw (Variables|Default|GetPlayerDeck))
  (Default|StartDraw (Variables|Default|GetEnemyDeck))
  (Utilities|FlowControl|Delay 3.5)
  (CallFunction|PhaseTransition "(R=0.000000,G=0.500000,B=1.000000,A=1.000000)" "Player Turn")
  (CallFunction|DrawPhase))

(event Custom|AIPlayCard
  (bind _enemy (Variables|Default|GetEnemy))
  (Utilities|Array|Clear (Variables|Default|GetAvailableSlots))
  (for _array_element (Variables|Default|GetEnemySlots)
    (Utilities|IsValid (Variables|/Game/Blueprints/SlotBP.SlotBP_C|GetPlacedCard _array_element)
      (:Is%20Not%20Valid
        (Utilities|Array|Add (Variables|Default|GetAvailableSlots) _array_element))))
  (if (and (> (Utilities|Array|Length (Variables|/Game/Blueprints/PlayerBP.PlayerBP_C|GetHandCards (Variables|Default|GetEnemy))) 0) (> (Utilities|Array|Length (Variables|Default|GetAvailableSlots)) 0))
    (Variables|/Game/Blueprints/PlayerBP.PlayerBP_C|SetCurrentCard _enemy (.OutItem (Utilities|Array|Random (Variables|/Game/Blueprints/PlayerBP.PlayerBP_C|GetHandCards _enemy))))
    (Default|PlaceCard (Variables|Default|GetEnemy) (.OutItem (Utilities|Array|Random (Variables|Default|GetAvailableSlots))))))

(event EventBeginPlay
  (Utilities|FlowControl|Delay 0.5)
  (CallFunction|StartPhase))

(event Collision|EventActorBeginOverlap
  (params (OtherActor :type Actor%20Object%20Reference)))

(event EventTick
  (params (DeltaSeconds :type Float%20%28single-precision%29)))

(fn ConstructionScript)